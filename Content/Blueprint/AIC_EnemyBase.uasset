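; AIC_EnemyBase is an AI controller Blueprint for enemies that runs the BT_Enemy_Base behavior tree when it possesses a pawn.
; On possession it puts the AI into a passive state by writing an AI state enum to the Blackboard.
; SetStateAsAttacking stores the given attack target in the Blackboard and switches that enum to attacking.
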(event EventPossess
  (params (PossessedPawn :type Pawn%20Object%20Reference))
  (AI|RunBehaviorTree "/Game/Blueprint/BT_Enemy_Base.BT_Enemy_Base")
  (CallFunction|SetStateasPassive))

(fn ConstructionScript)

(fn SetStateasPassive
  (AI|Components|Blackboard|SetValueasEnum (Variables|Default|GetBlackboard) (Variables|Default|GetAIStateName) (Utilities|Enum|LiteralenumEnum_AIState "NewEnumerator0")))

(fn SetStateasAttacking
  (params (AttackTarget :type Actor%20Object%20Reference))
  (AI|Components|Blackboard|SetValueasObject (Variables|Default|GetBlackboard) (Variables|Default|GetAttackTargetKeyName) AttackTarget)
  (AI|Components|Blackboard|SetValueasEnum (Variables|Default|GetBlackboard) (Variables|Default|GetAIStateName) (Utilities|Enum|LiteralenumEnum_AIState "NewEnumerator1")))