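; BP_PatrolRoute is an actor that defines a patrol path through the points of its Route spline.
; GetSplinePointAsWorldPos returns the world location of the spline point at the current PatrolIndex.
; IncrementPatroRoute steps the index by Direction, flipping it at the last and first points so the route runs back and forth instead of looping.
; The route stores this progress itself and moves nothing.
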(event Custom|IncrementPatroRoute
  ;[0.15 0.15 0.15 0.5] 判断Index是否到最后一个点了
  (bind _output_get (Variables|Default|SetPatrolIndex (+ (Variables|Default|GetPatrolIndex) (Variables|Default|GetDirection))))
  (if (== _output_get (- (Spline|GetNumberOfSplinePoints (Variables|Default|GetRoute)) 1))
    (Variables|Default|SetDirection -1)
    (elif (== (Variables|Default|GetPatrolIndex) 0)
      (Variables|Default|SetDirection 1))))

(fn ConstructionScript)

(fn GetSplinePointasWorldPos
  (return (Spline|GetLocationatSplinePoint (Variables|Default|GetRoute) (Variables|Default|GetPatrolIndex) "World")))